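; AI character Blueprint that appears to be a shopper NPC, able to be mugged and removed from the game.
; Mug sets BeingMugged and raises the MoveFail flag on the controller's blackboard.
; AllDone decrements the game manager's active shopper count, resets its spawn cooldown, then destroys the actor.
; The event graph holds only disabled default events, so the Blueprint runs no per-tick logic of its own.
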(event EventBeginPlay
  (|CallParentFunction) ; This node is disabled and will not be called.\nDrag off pins to build functionality.
)

(event Collision|EventActorBeginOverlap
  (params (OtherActor :type Actor%20Object%20Reference))
  (|CallParentFunction OtherActor) ; This node is disabled and will not be called.\nDrag off pins to build functionality.
)

(event EventTick
  (params (DeltaSeconds :type Float%20%28single-precision%29))
  (|CallParentFunction DeltaSeconds) ; This node is disabled and will not be called.\nDrag off pins to build functionality.
)

(fn ConstructionScript
  (|CallParentFunction))

(fn Mug
  (Variables|Default|SetBeingMugged true)
  (AI|Components|Blackboard|SetValueasBool (AI|GetBlackboard (Pawn|GetController)) (Utilities|Name|MakeLiteralName "MoveFail") true))

(fn AllDone
  (bind _man (CallFunction|GetGameManager))
  (Math|Integer|DecrementInt (Variables|/Game/Blueprints/GameManager.GameManager_C|GetActiveShoppers _man)
    (:%20%20
      (Variables|/Game/Blueprints/GameManager.GameManager_C|SetSpawnCoolDown _man 1.0)
      (Actor|DestroyActor))))