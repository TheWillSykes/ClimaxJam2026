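; GameCamera is an actor that subtly turns to follow the player character while staying biased toward its initial facing.
; BeginPlay stores the starting rotation.
; Each Tick builds an upright look-at rotation toward the player, then blends it mostly back toward the stored rotation along the shortest path, so it only partially tracks the player without moving.
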(event EventBeginPlay
  (Variables|Default|SetOriginalRotation (Transformation|GetActorRotation)))

(event Collision|EventActorBeginOverlap
  (params (OtherActor :type Actor%20Object%20Reference)))

(event EventTick
  (params (DeltaSeconds :type Float%20%28single-precision%29))
  (Transformation|SetActorRotation (Math|Rotator|Lerp(Rotator) (Math|Rotator|MakeRotfromXZ (Math|Vector|Normalize (- (Transformation|GetActorLocation (CallFunction|GetPlayerCharacter)) (Transformation|GetActorLocation))) (Math|Vector|MakeVector 0.0 0.0 1.0)) (Variables|Default|GetOriginalRotation) 0.75 true)))

(fn ConstructionScript)