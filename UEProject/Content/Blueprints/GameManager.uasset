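; GameManager runs the game countdown and keeps the level populated with shoppers.
; Each Tick reduces TimeRemaining by delta time, clamped so it stops at zero.
; While ActiveShoppers is below three, Tick spawns one randomly chosen PoorShopper or RichShopper at the Exit's transform and increments the count.
; This graph only increments the count and takes no action when time runs out.
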(event EventBeginPlay)

(event Collision|EventActorBeginOverlap
  (params (OtherActor :type Actor%20Object%20Reference)))

(event EventTick
  (params (DeltaSeconds :type Float%20%28single-precision%29))
  (Variables|Default|SetTimeRemaining (Math|Float|Clamp(Float) (- (Variables|Default|GetTimeRemaining) DeltaSeconds) 0.0 1e+07))
  ;[0.15 0.15 0.15 0.5] Respawn shoppers
  (if (< (Variables|Default|GetActiveShoppers) 3)
    (Game|SpawnActorfromClass (select (Math|Random|RandomBool) "/Game/Blueprints/PoorShopper.PoorShopper_C" "/Game/Blueprints/RichShopper.RichShopper_C") (Transformation|GetActorTransform (CallFunction|GetExit)) "Undefined" "MultiplyWithRoot" 0 0)
    (Math|Integer|IncrementInt (Variables|Default|GetActiveShoppers))))

(fn ConstructionScript)